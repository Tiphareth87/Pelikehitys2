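; Base 2D side-scroller player character with axis movement, jumping, a health HUD, healing and death.
; Tick picks the flipbook from velocity and turns control rotation to face travel direction.
; Capsule hits on enemies use hit direction to either stomp-kill or damage the player, with knockback and a brief DoOnce debounce.
; Death disables input, detaches the camera, launches the physics-driven capsule without collision, then loads the menu after a delay.
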(event OnComponentHit(CapsuleComponent)
  (params (HitComponent :type Primitive%20Component%20Object%20Reference) (OtherActor :type Actor%20Object%20Reference) (OtherComp :type Primitive%20Component%20Object%20Reference) (NormalImpulse :type Vector :default "0, 0, 0") (Hit :type Hit%20Result%20Structure%20%28by%20ref%29))
  (bind _asbp_enemy_base (Utilities|Casting|CastToBP_EnemyBase OtherActor))
  (Variables|Default|SetHitEnemyRef _asbp_enemy_base)
  (Utilities|FlowControl|DoOnce false
    (:Completed
      (Variables|Default|SetHitDirection (Math|Vector|Normalize (- (.location Hit) (Transformation|GetActorLocation))))
      (Utilities|FlowControl|Sequence
        (:then_0
          (if (<= (.z (Variables|Default|GetHitDirection)) -0.25)
            ;[1 1 1] Damage enemy
            (CallFunction|CancleMovement)
            (Physics|AddImpulse (Variables|Character|GetCharacterMovement) (Math|Vector|MakeVector 0.0 0.0 (Variables|Floats|GetKnockBackForce)) true)
            (Game|Damage|ApplyDamage (Variables|Default|GetHitEnemyRef) (Variables|/Game/Blueprints/Enemies/BP_EnemyBase.BP_EnemyBase_C|GetHealth (Variables|Default|GetHitEnemyRef)) 0 0)
            (else
              ;[1 1 1] Damage Player
              (CallFunction|CancleMovement)
              (Physics|AddImpulse (Variables|Character|GetCharacterMovement) (Math|Vector|MakeVector (* (.x (Variables|Default|GetHitDirection)) (* -1.0 (Variables|Floats|GetKnockBackForce))) 0.0 (Variables|Floats|GetKnockBackForce)) true)
              (Game|Damage|ApplyDamage self (Variables|Floats|GetPlayerDamage) 0 0))))
        (:then_1
          (Utilities|FlowControl|Delay 0.1)
          (CallFunction|ResetHitCheck))))))

(event Custom|ResetHitCheck
  (bind _hitenemyref (Variables|Default|GetHitEnemyRef))
  (Utilities|FlowControl|DoOnce false) ; enters at Reset
)

(event EventBeginPlay
  (Variables|Default|SetMovementState "NewEnumerator4")
  (bind _returnvalue (UserInterface|CreateWidget "/Game/Blueprints/UI/WBP_PlayerHealth.WBP_PlayerHealth_C"))
  (bind _output_get (Variables|Default|SetHealthWidgetRef _returnvalue))
  (UserInterface|Viewport|AddtoViewport _output_get 0)
  (CallFunction|UpdateHealthWidget))

(event EventTick
  (params (DeltaSeconds :type Float%20%28single-precision%29))
  (Utilities|FlowControl|Sequence
    (:then_0
      (CallFunction|UpdateFlipbook))
    (:then_1
      (CallFunction|UpdatePlayerRotation))))

(event Game|Damage|EventAnyDamage
  (params (Damage :type Float%20%28single-precision%29) (DamageType :type Damage%20Type%20Object%20Reference) (InstigatedBy :type Controller%20Object%20Reference) (DamageCauser :type Actor%20Object%20Reference))
  (Audio|PlaySound2D "/Game/Assets/SFX/punch.punch" 1.0 1.0 0.0 0 0)
  (Variables|Floats|SetHealth (Math|Float|Clamp(Float) (- (Variables|Floats|GetHealth) Damage) 0.0 (Variables|Floats|GetDefault%20Health)))
  (CallFunction|UpdateHealthWidget)
  (if (and (<= (Variables|Floats|GetHealth) 0.0) (not (Variables|Default|GetbisDead)))
    (CallFunction|PlayerDied)
    (Audio|PlaySound2D "/Game/Assets/Sounds/Stun_Cue.Stun_Cue" 1.0 1.0 0.0 0 0)
    (Utilities|FlowControl|Delay 7.0)
    (Game|OpenLevel(byName) "MenuLevel")))

(event Input|ActionEvents|InputActionJump
  (params (Key :type Key%20Structure))
  ;[1 1 1] Control Jump
  (:Pressed
    (Audio|PlaySound2D "/Game/Assets/SFX/JumpSFX.JumpSFX" 1.0 1.0 0.0 0 0)
    (Character|Jump))
  (:Released
    (Character|StopJumping)))

(event Input|AxisEvents|InputAxisMoveRight
  (params (AxisValue :type Float%20%28single-precision%29))
  ;[1 1 1] Directial movement
  (Pawn|Input|AddMovementInput "1.000000, 0, 0" AxisValue false))

(fn ConstructionScript
  (Variables|Floats|SetHealth (Variables|Floats|GetDefault%20Health)))

(fn UpdateFlipbook
  (Variables|Default|SetMovementState (select (!= (Math|Vector|VectorLength (Transformation|GetVelocity)) 0.0) (select (AI|Components|NavMovement|IsFalling (Variables|Character|GetCharacterMovement)) (select (<= (.z (Transformation|GetVelocity)) 0.0) "NewEnumerator3" "NewEnumerator2") "NewEnumerator1") "NewEnumerator0"))
  (Sprite|SetFlipbook (Variables|Default|GetSprite) (Utilities|Select :Index (Variables|Default|GetMovementState) :NewEnumerator4 0 :NewEnumerator0 (Variables|FP|GetFP_Idle) :NewEnumerator1 (Variables|FP|GetFP_Run) :NewEnumerator2 (Variables|FP|GetFP_Jump) :NewEnumerator3 (Variables|FP|GetFP_Fall))))

(fn UpdatePlayerRotation
  (Math|Float|CompareFloat (.x (Transformation|GetVelocity)) 0.0
    (:>
      (Pawn|SetControlRotation (Game|GetPlayerController 0) (Math|Rotator|MakeRotator 0.0 0.0 0.0)))
    (:<
      (Pawn|SetControlRotation (Game|GetPlayerController 0) (Math|Rotator|MakeRotator 0.0 0.0 1.8e+02)))))

(fn PlayerDied
  (Variables|Default|SetbisDead true)
  (Input|DisableInput (Game|GetPlayerController 0))
  (CallFunction|CancleMovement)
  (Transformation|DetachFromComponent (Variables|Default|GetSpringArm) "KeepWorld" "KeepRelative" "KeepRelative" true)
  (Collision|SetCollisionResponsetoAllChannels (Variables|Collision|GetCapsuleComponent) "ECR_Ignore")
  (Physics|SetSimulatePhysics (Variables|Collision|GetCapsuleComponent) true)
  (Physics|AddImpulse (Variables|Collision|GetCapsuleComponent) (Math|Vector|MakeVector 0.0 -5.0 9e+02) "None" true))

(fn UpdateHealthWidget
  (Default|UpdateHealth (Variables|Default|GetHealthWidgetRef) (Variables|Floats|GetHealth) (Variables|Floats|GetDefault%20Health)))

(fn CancleMovement
  (Variables|/Script/Engine.MovementComponent|SetVelocity (Variables|Character|GetCharacterMovement) "0, 0, 0")
  (Components|Movement|StopMovementImmediately (Variables|Character|GetCharacterMovement))
  (Class|PrimitiveComponent|SetAllPhysicsLinearVelocity (Variables|Collision|GetCapsuleComponent) "0, 0, 0" false))

(fn AddHealth
  (params (HealAmount :type Float%20%28single-precision%29))
  (Variables|Floats|SetHealth (Math|Float|Clamp(Float) (+ (Variables|Floats|GetHealth) HealAmount) 0.0 (Variables|Floats|GetDefault%20Health)))
  (CallFunction|UpdateHealthWidget))